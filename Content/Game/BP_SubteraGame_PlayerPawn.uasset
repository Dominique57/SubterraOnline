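; Player pawn for SubteraGame that moves along world Y and Z from Enhanced Input left, right, up and down actions.
; Only the pawn matching player index 0 enables input, combining forward and backward vectors each Tick into MovePawnRPC.
; MoveXYZ normalizes that vector into a fixed, unswept per-frame offset without delta-time scaling, printing each move.
; The authority-based EnableInputIfLocal function is never called here.
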(event Custom|MovePawnRPC
  (params (Movement :type Vector))
  (CallFunction|MoveXYZ Movement))

(event Input|EnhancedActionEvents|EnhancedInputActionIA_SubteraGame_MoveLeft
  (params (ActionValue :type Boolean) (ElapsedSeconds :type Float%20%28double-precision%29) (TriggeredSeconds :type Float%20%28double-precision%29) (InputAction :type Input%20Action%20Object%20Reference :default "/Game/Game/Input/IA_SubteraGame_MoveLeft.IA_SubteraGame_MoveLeft"))
  (:Triggered
    (Variables|Default|SetBckwdMove (Math|Vector|MakeVector (.X (Math|Vector|BreakVector (Variables|Default|GetBckwdMove))) 1.0 (.Z (Math|Vector|BreakVector (Variables|Default|GetBckwdMove))))))
  (:Completed
    (Variables|Default|SetBckwdMove (Math|Vector|MakeVector (.X (Math|Vector|BreakVector (Variables|Default|GetBckwdMove))) 0.0 (.Z (Math|Vector|BreakVector (Variables|Default|GetBckwdMove)))))))

(event Input|EnhancedActionEvents|EnhancedInputActionIA_SubteraGame_MoveRight
  (params (ActionValue :type Boolean) (ElapsedSeconds :type Float%20%28double-precision%29) (TriggeredSeconds :type Float%20%28double-precision%29) (InputAction :type Input%20Action%20Object%20Reference :default "/Game/Game/Input/IA_SubteraGame_MoveRight.IA_SubteraGame_MoveRight"))
  (:Triggered
    (Variables|Default|SetFwdMove (Math|Vector|MakeVector (.X (Math|Vector|BreakVector (Variables|Default|GetFwdMove))) 1.0 (.Z (Math|Vector|BreakVector (Variables|Default|GetFwdMove))))))
  (:Completed
    (Variables|Default|SetFwdMove (Math|Vector|MakeVector (.X (Math|Vector|BreakVector (Variables|Default|GetFwdMove))) 0.0 (.Z (Math|Vector|BreakVector (Variables|Default|GetFwdMove)))))))

(event Input|EnhancedActionEvents|EnhancedInputActionIA_SubteraGame_MoveUp
  (params (ActionValue :type Boolean) (ElapsedSeconds :type Float%20%28double-precision%29) (TriggeredSeconds :type Float%20%28double-precision%29) (InputAction :type Input%20Action%20Object%20Reference :default "/Game/Game/Input/IA_SubteraGame_MoveUp.IA_SubteraGame_MoveUp"))
  (:Triggered
    (Variables|Default|SetFwdMove (Math|Vector|MakeVector (.X (Math|Vector|BreakVector (Variables|Default|GetFwdMove))) (.Y (Math|Vector|BreakVector (Variables|Default|GetFwdMove))) 1.0)))
  (:Completed
    (Variables|Default|SetFwdMove (Math|Vector|MakeVector (.X (Math|Vector|BreakVector (Variables|Default|GetFwdMove))) (.Y (Math|Vector|BreakVector (Variables|Default|GetFwdMove))) 0.0))))

(event Input|EnhancedActionEvents|EnhancedInputActionIA_SubteraGame_MoveDown
  (params (ActionValue :type Boolean) (ElapsedSeconds :type Float%20%28double-precision%29) (TriggeredSeconds :type Float%20%28double-precision%29) (InputAction :type Input%20Action%20Object%20Reference :default "/Game/Game/Input/IA_SubteraGame_MoveDown.IA_SubteraGame_MoveDown"))
  (:Triggered
    (Variables|Default|SetBckwdMove (Math|Vector|MakeVector (.X (Math|Vector|BreakVector (Variables|Default|GetBckwdMove))) (.Y (Math|Vector|BreakVector (Variables|Default|GetBckwdMove))) 1.0)))
  (:Completed
    (Variables|Default|SetBckwdMove (Math|Vector|MakeVector (.X (Math|Vector|BreakVector (Variables|Default|GetBckwdMove))) (.Y (Math|Vector|BreakVector (Variables|Default|GetBckwdMove))) 0.0))))

(event EventBeginPlay
  (bind _returnvalue (Game|GetPlayerController 0))
  (if (== (Game|Player|GetPlayerPawn 0) self)
    (Input|AddMappingContext (PlayerController|LocalPlayerSubsystems|GetEnhancedInputLocalPlayerSubsystem _returnvalue) (Variables|Default|GetMapping%20Context) 0 "(bIgnoreAllPressedKeysUntilRelease=True,bForceImmediately=False)")
    (Input|EnableInput _returnvalue)
    (else
      (Input|DisableInput _returnvalue))))

(event EventTick
  (params (DeltaSeconds :type Float%20%28single-precision%29))
  (if (== (Game|Player|GetPlayerPawn 0) self)
    (CallFunction|MovePawnRPC (- (Variables|Default|GetFwdMove) (Variables|Default|GetBckwdMove)))))

(fn ConstructionScript)

(fn EnableInputifLocal
  (bind _returnvalue (Game|GetPlayerController 0))
  (Networking|SwitchHasAuthority
    (:Authority
      (Input|EnableInput _returnvalue))
    (:Remote
      (Input|DisableInput _returnvalue))))

(fn MoveXYZ
  (params (Movement :type Vector))
  (bind _returnvalue (Math|Float|MakeLiteralFloat 1e+01))
  (bind _returnvalue_2 (Math|Vector|Normalize Movement))
  (bind _returnvalue_3 (* _returnvalue_2 _returnvalue))
  (Math|Float|CompareFloat (Math|Vector|VectorLength _returnvalue_3) 0.1
    (:>
      (Transformation|AddActorWorldOffset _returnvalue_3)
      (Development|PrintString (Utilities|String|Append (Utilities|GetDisplayName self) (Utilities|String|ToString(Vector) _returnvalue_3))))))